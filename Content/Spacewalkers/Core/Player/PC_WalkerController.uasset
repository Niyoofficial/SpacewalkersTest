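; PC_WalkerController is the Spacewalkers player controller that relays module actions to the game board.
; On BeginPlay it caches the game mode as BP_MainGameMode.
; Its events for dropping a template, leveling up and fixing a module pass grid coordinates, plus the module class when adding, to the game mode's GameBoard.
; The controller holds no board logic itself, only forwarding each action.
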(event Custom|TemplateDropped
  (params (X :type Integer) (Y :type Integer) (Class :type Module%20Base%20Class%20Reference))
  (Class|GameBoard|AddModule (Variables|/Script/SpaceWalkersTest.MainGameMode|GetGameBoard (Variables|Default|GetGameMode)) Class X Y))

(event Custom|ModuleFix
  (params (X :type Integer) (Y :type Integer))
  (Class|GameBoard|FixModule (Variables|/Script/SpaceWalkersTest.MainGameMode|GetGameBoard (Variables|Default|GetGameMode)) X Y))

(event Custom|ModuleLevelUp
  (params (X :type Integer) (Y :type Integer))
  (Class|GameBoard|LevelUpModule (Variables|/Script/SpaceWalkersTest.MainGameMode|GetGameBoard (Variables|Default|GetGameMode)) X Y))

(event EventBeginPlay
  (bind _asbp_main_game_mode (Utilities|Casting|CastToBP_MainGameMode (Game|GetGameMode)))
  (Variables|Default|SetGameMode _asbp_main_game_mode))

(fn ConstructionScript)