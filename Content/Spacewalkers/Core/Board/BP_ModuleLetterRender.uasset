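; BP_ModuleLetterRender renders a single letter mesh into its own render target.
; The construction script assigns the mesh to Letter and limits the scene capture to that component.
; BeginPlay creates a mipmapped render target for the capture and sets the rotation timeline's rate from RotateSpeed.
; That timeline maps its alpha to a full yaw turn of the letter, though nothing in the graph starts it.
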(event EventBeginPlay
  (Components|Timeline|SetPlayRate (Variables|Default|GetRotateTimeline) (/ 1.0 (Variables|Default|GetRotateSpeed)))
  (bind _returnvalue (Rendering|CreateRenderTarget2D 1024 1024 "RTF_RGBA16f" "(R=0.000000,G=0.000000,B=0.000000,A=1.000000)" true))
  (bind _output_get (Variables|Default|SetRenderTarget _returnvalue))
  (Variables|/Script/Engine.SceneCaptureComponent2D|SetTextureTarget (Variables|Default|GetSceneCaptureComponent2D) _output_get))

(fn ConstructionScript
  (Rendering|SceneCapture|ShowOnlyComponent (Variables|Default|GetSceneCaptureComponent2D) (Variables|Default|GetLetter))
  (Components|StaticMesh|SetStaticMesh (Variables|Default|GetLetter) (Variables|Default|GetMesh)))